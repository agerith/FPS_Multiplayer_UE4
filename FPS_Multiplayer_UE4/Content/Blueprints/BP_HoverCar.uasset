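; BP_HoverCar is a drivable hover car pawn moved by physics forces on its mesh.
; Four hover components are initialized with CarMesh on BeginPlay.
; MoveForward and MoveRight axis inputs call server events that apply forward force and yaw torque, without delta-time scaling.
; PossessCar only prints the instigator's name; the possession handoff through BP_PlayerController is disconnected and never runs.
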(event `self.ReceiveBeginPlay`
  (`/Game/Blueprints/SC_HoverComponent.InitComponent` (`self.SC_HoverComponent2`) (`self.CarMesh`))
  (`/Game/Blueprints/SC_HoverComponent.InitComponent` (`self.SC_HoverComponent3`) (`self.CarMesh`))
  (`/Game/Blueprints/SC_HoverComponent.InitComponent` (`self.SC_HoverComponent`) (`self.CarMesh`))
  (`/Game/Blueprints/SC_HoverComponent.InitComponent` (`self.SC_HoverComponent1`) (`self.CarMesh`)))

(event `InputAxis|MoveForward`
  (params (AxisValue :type "Float (single-precision)"))
  (`self.MoveForward_Server` AxisValue))

(event `MoveForward_Server`
  (params (AxisValue :type "Float (double-precision)"))
  (`PrimitiveComponent.AddForce` (`self.CarMesh`) (* (* (`SceneComponent.GetForwardVector` (`self.CarMesh`)) 300000.0) AxisValue) "None" false))

(event `InputAxis|MoveRight`
  (params (AxisValue :type "Float (single-precision)"))
  (`self.MoveRight_Server` AxisValue))

(event `MoveRight_Server`
  (params (AxisValue :type "Float (double-precision)"))
  (`PrimitiveComponent.AddTorqueInRadians` (`self.CarMesh`) (`KismetMathLibrary.MakeVector` 0.0 0.0 (* AxisValue 4500000.0)) "None" false))

(event `self.PossessCar`
  (params (InstigatorPawn :type "Pawn Object Reference"))
  (`KismetSystemLibrary.PrintString` (`KismetSystemLibrary.GetDisplayName` InstigatorPawn)))

(fn `UserConstructionScript`)