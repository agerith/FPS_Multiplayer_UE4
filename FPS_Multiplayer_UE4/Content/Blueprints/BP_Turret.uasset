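; Turret actor that acquires a pawn through PawnSensing sight or a server-only sphere overlap.
; Tick is built to yaw the turret toward its target and call Shoot, which spawns projectiles at the head socket after a Delay, once sight has enabled firing.
; CheckDistance gates this and otherwise drops the target, but its range comparison is left unconnected.
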(event `self.ReceiveTick`
  (params (DeltaSeconds :type "Float (single-precision)"))
  (`self.PawnTarget`
    (:`then`
      (if (`self.EnemyInrange`)
        (if (`self.CheckDistance`)
          (`self.UpdateRotation`)
          (`self.Shoot`)
          (else
            (set `self.PawnTarget` null)
            (set `self.EnemyInrange` false)))))
    (:`else`)))

(event `UpdateRotation`
  (bind (_returnvalue_roll _returnvalue_pitch _returnvalue_yaw) (`KismetMathLibrary.BreakRotator` (`KismetMathLibrary.FindLookAtRotation` (`SceneComponent.K2_GetComponentLocation` (`self.DefaultSceneRoot`)) (`self.K2_GetActorLocation` (`self.PawnTarget`)))))
  (`SceneComponent.K2_SetWorldRotation` (`self.DefaultSceneRoot`) (`KismetMathLibrary.RInterpTo_Constant` (`SceneComponent.K2_GetComponentRotation` (`self.DefaultSceneRoot`)) (`KismetMathLibrary.MakeRotator` 0.0 0.0 _returnvalue_yaw) (`GameplayStatics.GetWorldDeltaSeconds`) (`self.RotationSpeed`)) false false))

(event `self.PawnSensing.OnSeePawn`
  (params (Pawn :type "Pawn Object Reference"))
  (set `self.PawnTarget` Pawn)
  (set `self.EnemyInrange` true)
  (set `self.Fire` true))

(event `self.PawnSensing.OnHearNoise`
  (params (Instigator :type "Pawn Object Reference") (Location :type "Vector Structure (by ref)") (Volume :type "Float (single-precision)")))

(event `Shoot`
  (if (`self.Fire`)
    (`KismetSystemLibrary.Delay` (`self.FireInterval`))
    (`|SpawnActorFromClass` "/Game/Blueprints/TurretProjectile.TurretProjectile_C" (`SceneComponent.GetSocketTransform` (`self.Turret_Top_001_FBX`) "head" "RTS_World") "AlwaysSpawn" "OverrideRootScale" null null)))

(event `self.Sphere.OnComponentBeginOverlap`
  (params (OverlappedComponent :type "PrimitiveComponent Object Reference") (OtherActor :type "Actor Object Reference") (OtherComp :type "PrimitiveComponent Object Reference") (OtherBodyIndex :type Integer) (bFromSweep :type Boolean) (SweepResult :type "HitResult Structure (by ref)"))
  (bind _aspawn (cast `Pawn` OtherActor))
  (`/Engine/EditorBlueprintResources/ActorMacros.Switch Has Authority`
    (:`Authority`
      (set `self.PawnTarget` _aspawn)
      (set `self.EnemyInrange` true))))

(fn `UserConstructionScript`)