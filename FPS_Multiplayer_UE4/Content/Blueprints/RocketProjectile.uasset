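; Rocket projectile that damages a first-person character on impact or explodes against anything else, with optional homing.
; Its first collision hit either calls DealDamage on the character or fires a radial impulse and spawns an emitter, then destroys the rocket.
; A HomingMissile event switches the projectile movement to homing on a valid target's root component with high acceleration.
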(event `self.CollisionComponent.OnComponentHit`
  (params (HitComponent :type "PrimitiveComponent Object Reference") (OtherActor :type "Actor Object Reference") (OtherComp :type "PrimitiveComponent Object Reference") (NormalImpulse :type "Vector Structure") (Hit :type "HitResult Structure (by ref)"))
  (bind _explosionforce (`self.ExplosionForce`))
  (`/Engine/EditorBlueprintResources/StandardMacros.DoOnce` false
    (:`Completed`
      (bind _asfirst_person_character (cast `/Game/FirstPersonCPP/Blueprints/FirstPersonCharacter` OtherActor)
        (:`then`
          (`TestRyseUpCharacter.DealDamage` _asfirst_person_character Hit NormalImpulse 25.0 "/Game/DamageTypes/DmgType_RifflePickup.DmgType_RifflePickup_C" _asfirst_person_character)
          (`self.K2_DestroyActor`))
        (:`CastFailed`
          (`RadialForceComponent.FireImpulse` _explosionforce)
          (`GameplayStatics.SpawnEmitterAtLocation` null (`SceneComponent.K2_GetComponentLocation` _explosionforce))
          (`self.K2_DestroyActor`))))))

(event `HomingMissile`
  (params (TargetToHit :type "Actor Object Reference"))
  (bind _projectile (`self.Projectile`))
  (`/Engine/EditorBlueprintResources/StandardMacros.IsValid` TargetToHit
    (:`Is Valid`
      (set `ProjectileMovementComponent.HomingTargetComponent` (`Actor.RootComponent` TargetToHit) _projectile)
      (set `ProjectileMovementComponent.bIsHomingProjectile` true _projectile)
      (set `ProjectileMovementComponent.HomingAccelerationMagnitude` 25000.0 _projectile))))

(fn `UserConstructionScript`)