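; Scene component that shows a colored screen marker tracking its world location, as an off-screen target indicator for the first player.
; BeginPlay creates a W_ImageOffscreen widget; InitColor recolors it and RemoveWidget removes it.
; Tick projects the location to screen, clamps the widget within an edge margin, and rotates it away from center when outside.
; Paired DoOnce gates swap square and arrow images only when crossing that margin.
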(event `InitColor`
  (params (Color :type "LinearColor Structure"))
  (bind _output_get (set `self.Color` Color))
  (set `/Game/HUD/UMG/W_ImageOffscreen.Color` _output_get (`self.OffScreen_Wiget`)))

(event `self.ReceiveBeginPlay`
  (bind _returnvalue (`|CreateWidget` "/Game/HUD/UMG/W_ImageOffscreen.W_ImageOffscreen_C" null (`self.Color`)))
  (set `self.OffScreen_Wiget` _returnvalue)
  (`UserWidget.AddToViewport` _returnvalue 0))

(event `RemoveWidget`
  (`Widget.RemoveFromParent` (`self.OffScreen_Wiget`)))

(event `self.ReceiveTick`
  (params (DeltaSeconds :type "Float (single-precision)"))
  (bind (_returnvalue_x _returnvalue_y) (`KismetMathLibrary.BreakVector2D` (`WidgetLayoutLibrary.GetViewportSize`)))
  (bind (_returnvalue_x_2 _returnvalue_y_2) (`KismetMathLibrary.BreakVector2D` (`WidgetLayoutLibrary.GetViewportSize`)))
  (bind _offsetposition (`self.OffsetPosition`))
  (bind _offsetposition_2 (`self.OffsetPosition`))
  (bind _screenposition (`GameplayStatics.ProjectWorldToScreen` (`GameplayStatics.GetPlayerController` 0) (`self.K2_GetComponentLocation`)))
  (bind _returnvalue (- _returnvalue_y_2 (`self.OffsetPosition`)))
  (bind _returnvalue_2 (- _returnvalue_x_2 (`self.OffsetPosition`)))
  (bind _returnvalue_3 (`KismetMathLibrary.FClamp` (`.Y` (`KismetMathLibrary.BreakVector2D` _screenposition)) _offsetposition_2 _returnvalue))
  (bind _returnvalue_4 (`KismetMathLibrary.FClamp` (`KismetMathLibrary.BreakVector2D` _screenposition) _offsetposition_2 _returnvalue_2))
  (bind _returnvalue_5 (and (and (> (`KismetMathLibrary.BreakVector2D` _screenposition) _offsetposition) (< (`KismetMathLibrary.BreakVector2D` _screenposition) _returnvalue_2)) (and (> (`.Y` (`KismetMathLibrary.BreakVector2D` _screenposition)) _offsetposition) (< (`.Y` (`KismetMathLibrary.BreakVector2D` _screenposition)) _returnvalue))))
  (`UserWidget.SetPositionInViewport` (`self.OffScreen_Wiget`) (`KismetMathLibrary.MakeVector2D` _returnvalue_4 _returnvalue_3) true)
  (`Widget.SetRenderAngle` (`/Game/HUD/UMG/W_ImageOffscreen.Image_70` (`self.OffScreen_Wiget`)) (`KismetMathLibrary.SelectFloat` 0.0 (`KismetMathLibrary.RadiansToDegrees` (`KismetMathLibrary.Atan2` (- _returnvalue_3 (/ _returnvalue_y 2.0)) (- _returnvalue_4 (/ _returnvalue_x 2.0)))) _returnvalue_5))
  (if _returnvalue_5
    (`/Engine/EditorBlueprintResources/StandardMacros.DoOnce` false :!label _label
      (:`Completed`
        (`Image.SetBrush` (`/Game/HUD/UMG/W_ImageOffscreen.Image_70` (`self.OffScreen_Wiget`)) (make `SlateBrush` (100.0 100.0) (struct) (struct :`SpecifiedColor` (struct :`R` 1.0 :`G` 1.0 :`B` 1.0 :`A` 1.0) :`ColorUseRule` "UseColor_Specified") "/Game/HUD/UMG/651662_square_512x512.651662_square_512x512"))
        (goto _label_2 :!via `Reset`)))
    (else
      (`/Engine/EditorBlueprintResources/StandardMacros.DoOnce` false :!label _label_2
        (:`Completed`
          (`Image.SetBrush` (`/Game/HUD/UMG/W_ImageOffscreen.Image_70` (`self.OffScreen_Wiget`)) (make `SlateBrush` (100.0 100.0) (struct) (struct :`SpecifiedColor` (struct :`R` 1.0 :`G` 1.0 :`B` 1.0 :`A` 1.0) :`ColorUseRule` "UseColor_Specified") "/Game/HUD/UMG/if_icon-ios7-arrow-forward_211688.if_icon-ios7-arrow-forward_211688"))
          (goto _label :!via `Reset`))))))